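; VR pawn for Oculus hand tracking that supports dictating text onto Sticky notes.
; On BeginPlay it sets eye-level tracking and snaps finger colliders to both hands' bone sockets, plus a widget palette to the left wrist.
; A Sticky entering VoiceCollider starts voice transcription, and leaving it writes the result into that note.
; It also has a Sticky pick-up helper, debug right-hand pinch readouts and hold-to-record mic capture to timestamped WAV files.
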(event `self.ReceiveBeginPlay`
  (`HeadMountedDisplayFunctionLibrary.SetTrackingOrigin` "Eye")
  (`self.PlaceCylinders`))

(event `InputAxisKey|OculusHand_Right_IndexPinchStrength`
  (params (AxisValue :type "Float (single-precision)"))
  ;[1 1 1] Pinch Texts
  (if (`self.DebugEnabled`)
    (`TextRenderComponent.K2_SetText` (`self.IndexPinch`) (`KismetTextLibrary.Conv_StringToText` (`KismetStringLibrary.Concat_StrStr` "Index: " (`KismetStringLibrary.Conv_DoubleToString` AxisValue))))))

(event `InputAxisKey|OculusHand_Right_ThumbPinchStrength`
  (params (AxisValue :type "Float (single-precision)"))
  ;[1 1 1] Pinch Texts
  (if (`self.DebugEnabled`)
    (`TextRenderComponent.K2_SetText` (`self.ThumbPinch`) (`KismetTextLibrary.Conv_StringToText` (`KismetStringLibrary.Concat_StrStr` "Thumb: " (`KismetStringLibrary.Conv_DoubleToString` AxisValue))))))

(event `InputAxisKey|OculusHand_Right_MiddlePinchStrength`
  (params (AxisValue :type "Float (single-precision)"))
  ;[1 1 1] Pinch Texts
  (if (`self.DebugEnabled`)
    (`TextRenderComponent.K2_SetText` (`self.MiddlePinch`) (`KismetTextLibrary.Conv_StringToText` (`KismetStringLibrary.Concat_StrStr` "Middle: " (`KismetStringLibrary.Conv_DoubleToString` AxisValue))))))

(event `InputAxisKey|OculusHand_Right_RingPinchStrength`
  (params (AxisValue :type "Float (single-precision)"))
  ;[1 1 1] Pinch Texts
  (if (`self.DebugEnabled`)
    (`TextRenderComponent.K2_SetText` (`self.RingPinch`) (`KismetTextLibrary.Conv_StringToText` (`KismetStringLibrary.Concat_StrStr` "Ring: " (`KismetStringLibrary.Conv_DoubleToString` AxisValue))))))

(event `InputAxisKey|OculusHand_Right_PinkPinchStrength`
  (params (AxisValue :type "Float (single-precision)"))
  ;[1 1 1] Pinch Texts
  (if (`self.DebugEnabled`)
    (`TextRenderComponent.K2_SetText` (`self.PinkyPinch`) (`KismetTextLibrary.Conv_StringToText` (`KismetStringLibrary.Concat_StrStr` "Pinky: " (`KismetStringLibrary.Conv_DoubleToString` AxisValue))))))

(event `InputAction|ToggleAudioCapture`
  (params (Key :type "Key Structure"))
  (bind (_returnvalue_year _returnvalue_month _returnvalue_day _returnvalue_hour _returnvalue_minute _returnvalue_second) (`KismetMathLibrary.BreakDateTime` (`KismetMathLibrary.Now`)))
  ;[1 1 1] Audio Capture
  (:`Pressed`
    (`KismetSystemLibrary.PrintString` "Starting Recording")
    (`AudioMixerBlueprintLibrary.StartRecordingOutput` 30.0 "/Game/Audio/MicInput.MicInput"))
  (:`Released`
    (`KismetSystemLibrary.PrintString` "Ending Recording")
    (`AudioMixerBlueprintLibrary.StopRecordingOutput` "WavFile" (`KismetTextLibrary.Conv_TextToString` (`|FormatText` "Recording_{Hour}-{Minute}-{Second}" _returnvalue_hour _returnvalue_minute _returnvalue_second)) (`KismetTextLibrary.Conv_TextToString` (`|FormatText` "{base}{sub}" (`KismetSystemLibrary.GetProjectDirectory`) (`self.Directory`))) null null)))

(event `PlaceCylinders`
  (`|ExecutionSequence`
    (:`then_0`
      ;[1 1 1] Right Hand
      (`SceneComponent.K2_AttachToComponent` (`self.IndexCollider_R`) (`self.OculusHand_R`) "Index3" "SnapToTarget" "KeepRelative" "KeepRelative" true)
      (`SceneComponent.K2_AttachToComponent` (`self.MiddleCollider_R`) (`self.OculusHand_R`) "Middle3" "SnapToTarget" "KeepRelative" "KeepRelative" true)
      (`SceneComponent.K2_AttachToComponent` (`self.ThumbCollider_R`) (`self.OculusHand_R`) "Thumb3" "SnapToTarget" "KeepRelative" "KeepRelative" true))
    (:`then_1`
      ;[1 1 1] Left Hand
      (`SceneComponent.K2_AttachToComponent` (`self.IndexCollider_L`) (`self.OculusHand_L`) "Index3" "SnapToTarget" "KeepRelative" "KeepRelative" true)
      (`SceneComponent.K2_AttachToComponent` (`self.MiddleCollider_L`) (`self.OculusHand_L`) "Middle3" "SnapToTarget" "KeepRelative" "KeepRelative" true)
      (`SceneComponent.K2_AttachToComponent` (`self.ThumbCollider_L`) (`self.OculusHand_L`) "Thumb3" "SnapToTarget" "KeepRelative" "KeepRelative" true))
    (:`then_2`
      ;[1 1 1] Widget Palette
      (`SceneComponent.K2_AttachToComponent` (`self.ChildActor`) (`self.OculusHand_L`) "Wrist Root" "SnapToTarget" "KeepRelative" "KeepRelative" true))))

(event `self.VoiceCollider.OnComponentBeginOverlap`
  (params (OverlappedComponent :type "PrimitiveComponent Object Reference") (OtherActor :type "Actor Object Reference") (OtherComp :type "PrimitiveComponent Object Reference") (OtherBodyIndex :type Integer) (bFromSweep :type Boolean) (SweepResult :type "HitResult Structure (by ref)"))
  ;[1 1 1] Voice Start
  (cast `/Game/Actors/Sticky` OtherActor)
  (`/Game/Components/VoiceTranscriptionComponent.StartRecording` (`self.VoiceTranscriptionComponent`)))

(event `self.VoiceCollider.OnComponentEndOverlap`
  (params (OverlappedComponent :type "PrimitiveComponent Object Reference") (OtherActor :type "Actor Object Reference") (OtherComp :type "PrimitiveComponent Object Reference") (OtherBodyIndex :type Integer))
  ;[1 1 1] Voice Start
  (bind _assticky (cast `/Game/Actors/Sticky` OtherActor))
  (bind _transcribed_text (`/Game/Components/VoiceTranscriptionComponent.EndRecording` (`self.VoiceTranscriptionComponent`)))
  (`/Game/Actors/Widget.UpdateContent` _assticky _transcribed_text))

(fn `PickUpSticky`
  (params (Sticky :type "/Game/Actors/Sticky Object Reference") (OverlappedComponent :type "SceneComponent Object Reference"))
  (`self.K2_AttachToComponent` Sticky OverlappedComponent "None" "SnapToTarget" "KeepRelative" "KeepRelative" true))

(fn `UserConstructionScript`)