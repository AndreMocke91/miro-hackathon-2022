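; Miro API wrapper Blueprint that creates and fetches sticky notes on a Miro board.
; Init loads the access token from a credential file in the project directory, broadcasts InitializationComplete with the success flag, and stores the board ID.
; Requests bind their result delegates after being issued; fetched JSON is marshalled and rebroadcast through GetStickiesResultComplete, while the create result is ignored.
; Token load results are printed, including the token itself.
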(event `Init`
  (params (BoardId :type String))
  (`|ExecutionSequence`
    (:`then_0`
      (`self.LoadApiTokenFromFile`))
    (:`then_1`
      (set `self.Board ID` BoardId))))

(event `CreateStickyEvent`
  (params (Content :type Text) (xPos :type "Float (double-precision)") (yPos :type "Float (double-precision)"))
  ;[1 1 1] CreateSticky
  ;;[1 1 1] Actual call
  (`self.CreateSticky` (make `CreateStickyRequest` (`self.Board ID`) (`self.API Access Token`) (`KismetTextLibrary.Conv_TextToString` Content) xPos yPos))
  (add `self.OnCreateStickyResult` (delegate `CreatStickyResult`)))

(event `CreatStickyResult` :!signature `self.OnCreateStickyResult`
  (params (CreateStickyResult :type String))
  ;[1 1 1] CreateSticky
  ;;[1 1 1] Actual call
)

(event `GetStickiesEvent`
  ;[1 1 1] GetStickies
  (`self.GetStickies` (make `GetStickiesRequest` (`self.Board ID`) (`self.API Access Token`)))
  (add `self.OnGetStickiesResult` (delegate `GetStickiesResult`)))

(event `GetStickiesResult` :!signature `self.OnGetStickiesResult`
  (params (GetStickiesJsonResult :type String))
  ;[1 1 1] GetStickies
  (bind _returnvalue (`self.FMarshalGetStickiesResult` GetStickiesJsonResult))
  (`self.GetStickiesResultComplete` _returnvalue))

(fn `LoadApiTokenFromFile`
  (bind _returnvalue (`KismetStringLibrary.Concat_StrStr` (`KismetSystemLibrary.GetProjectDirectory`) (`self.CredentialFileName`)))
  (bind (_output _returnvalue_2) (`JsonBlueprintUtilities.LoadApiToken` _returnvalue))
  (if _returnvalue_2
    (bind _output_get (set `self.API Access Token` _output))
    (`|ExecutionSequence`
      (:`then_0`
        (`KismetSystemLibrary.PrintString` (`KismetStringLibrary.Concat_StrStr` "Using API access token: " _output_get)))
      (:`then_1`
        (`self.InitializationComplete` _returnvalue_2 :!label _label)))
    (else
      (`|ExecutionSequence`
        (:`then_0`
          (goto _label))
        (:`then_1`
          (`KismetSystemLibrary.PrintString` (`KismetStringLibrary.Concat_StrStr` "Unable to load API access token from file: " _returnvalue)))))))